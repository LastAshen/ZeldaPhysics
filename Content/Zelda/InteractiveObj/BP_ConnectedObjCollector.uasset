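; BP_ConnectedObjCollector keeps a group of connected interactive objects and switches them on and off together.
; AddNew and Remove maintain the unique ConnectedObjects list.
; ToggleWorkingState flips the shared OnWorking flag, then calls Work or Shutdown on every object in the list to match the new state.
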(event Custom|AddNew
  (params (New :type BP%20Connectable%20Actor%20Object%20Reference))
  (Utilities|Array|AddUnique (Variables|Default|GetConnectedObjects) New))

(event Custom|Remove
  (params (Obj :type BP%20Connectable%20Actor%20Object%20Reference))
  (Utilities|Array|RemoveItem (Variables|Default|GetConnectedObjects) Obj))

(event Custom|ToggleWorkingState
  (Variables|Default|SetbOnWorking (not (Variables|Default|GetbOnWorking)))
  (for _array_element (Variables|Default|GetConnectedObjects)
    (if (Variables|Default|GetbOnWorking)
      (Default|Work _array_element)
      (else
        (Default|Shutdown _array_element)))))