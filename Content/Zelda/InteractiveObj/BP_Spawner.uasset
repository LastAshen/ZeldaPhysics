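; BP_Spawner is an interactive object that spawns an actor of a configurable class and shows a configurable text label.
; When one specific cylinder component overlaps its trigger box, it spawns the class, if valid, at a second cylinder's location and rotation.
; That second cylinder spins continuously on Tick, so the spawned actor's rotation follows the current spin.
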(event OnComponentBeginOverlap(Box_D57883F9)
  (params (OverlappedComponent :type Primitive%20Component%20Object%20Reference) (OtherActor :type Actor%20Object%20Reference) (OtherComp :type Primitive%20Component%20Object%20Reference) (OtherBodyIndex :type Integer) (bFromSweep :type Boolean) (SweepResult :type Hit%20Result%20Structure%20%28by%20ref%29))
  (bind _spawnedactorclass (Variables|Default|GetSpawnedActorClass))
  (bind _cylinder_12a03c78 (Variables|Default|GetCylinder_12A03C78))
  (bind _returnvalue (Transformation|GetWorldTransform _cylinder_12a03c78))
  (if (== OtherComp (Variables|Default|GetCylinder_12A03C77))
    (if (Utilities|IsValidClass _spawnedactorclass)
      (Game|SpawnActorfromClass _spawnedactorclass (Math|Transform|MakeTransform (.location _returnvalue) (.rotation _returnvalue) "1.000000,1.000000,1.000000") "Undefined" "MultiplyWithRoot" 0 0))))

(event EventBeginPlay
  (Rendering|Components|TextRender|SetText (Variables|Default|GetTextRender) (Variables|Default|GetText)))

(event Collision|EventActorBeginOverlap
  (params (OtherActor :type Actor%20Object%20Reference)))

(event EventTick
  (params (DeltaSeconds :type Float%20%28single-precision%29))
  (Transformation|AddLocalRotation (Variables|Default|GetCylinder_12A03C78) "0.000000,2.000000,0.000000" false false))

(fn ConstructionScript)