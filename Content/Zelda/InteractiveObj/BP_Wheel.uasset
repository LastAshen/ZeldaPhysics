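; BP_Wheel is a Zelda interactive object: a physics-driven wheel that can be switched between working and shut down.
; Work drives the physics constraint's angular velocity target on Z at RotateSpeed, clears the wheel's angular damping and wakes the body.
; Shutdown zeroes the velocity target and raises angular damping on the wheel to resist further spinning.
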(event EventWork
  (bind _wheel (Variables|Default|GetWheel))
  (Class|PhysicsConstraintComponent|SetAngularVelocityTarget (Variables|Default|GetPhysicsConstraint) (Math|Vector|MakeVector 0.0 0.0 (Variables|Default|GetRotateSpeed)))
  (Class|PrimitiveComponent|SetAngularDamping _wheel 0.0)
  (Class|PrimitiveComponent|WakeRigidBody _wheel "None"))

(event EventShutdown
  (Class|PhysicsConstraintComponent|SetAngularVelocityTarget (Variables|Default|GetPhysicsConstraint) (Math|Vector|MakeVector 0.0 0.0 0.0))
  (Class|PrimitiveComponent|SetAngularDamping (Variables|Default|GetWheel) 0.8))

(fn ConstructionScript
  (|CallParentFunction))