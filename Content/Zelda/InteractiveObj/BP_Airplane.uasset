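; BP_Airplane is a physics-driven interactive airplane whose engine power is switched on and off by Work and Shutdown events.
; Each tick, it pushes the propeller along its up vector with power divided by current speed, so thrust falls as speed rises.
; It also applies lift along the base's right vector, proportional to the base's speed along its up axis.
; Both forces are applied as acceleration changes, ignoring mass.
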(event Custom|PropellerForwardForce
  (bind _propeller (Variables|Default|GetPropeller))
  ;[1 1 1] Comment
  (Physics|AddForce _propeller (* (Math|Vector|GetUpVector _propeller) (Math|Float|SafeDivide (Variables|Default|GetPower) (Math|Float|Max(Float) (Math|Vector|VectorLength (Transformation|GetVelocity)) 1.0))) "None" true))

(event Custom|RiseForce
  (bind _base (Variables|Default|GetBase))
  (bind _base_2 (Variables|Default|GetBase))
  (bind _returnvalue (Math|Vector|GetUpVector _base))
  (bind _returnvalue_2 (Transformation|GetComponentVelocity _base))
  (bind _returnvalue_3 (Class|KismetMathLibrary|VectorProjectontoNormal _returnvalue_2 _returnvalue))
  (bind _returnvalue_4 (Math|Vector|VectorLength _returnvalue_3))
  ;[1 1 1] Comment
  (if (> _returnvalue_4 0.0)
    (Physics|AddForce _base_2 (* (Math|Vector|GetRightVector _base_2) (* _returnvalue_4 (Variables|Default|GetRiseForceConvertRate))) "None" true)))

(event EventWork
  (Variables|Default|SetPower 3e+04))

(event EventTick
  (params (DeltaSeconds :type Float%20%28single-precision%29))
  ;[1 1 1] Comment
  (CallFunction|PropellerForwardForce)
  (CallFunction|RiseForce))

(event EventShutdown
  (Variables|Default|SetPower 0.0))

(fn ConstructionScript)