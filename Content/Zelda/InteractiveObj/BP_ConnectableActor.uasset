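; Base actor for interactive objects that can be connected, with empty Work, Shutdown and GetMainPhysicsBody stubs.
; The construction script creates a BP_ConnectedObjCollector for each actor and registers the actor with it.
; On BeginPlay it maps every socket name on its primitive components to the owning component.
; Socket names must be unique across the actor, and duplicates print a red on-screen warning instead of being added.
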(event EventBeginPlay
  ;[1 1 1] Collect All Sockets to Meshes
  (for _array_element (Actor|GetComponentsByClass "/Script/Engine.PrimitiveComponent")
    (for _array_element_2 (Transformation|GetAllSocketNames _array_element)
      (if (Utilities|Map|Contains (Variables|Default|GetSocketNamesToMeshes) _array_element_2)
        (Development|PrintString (Utilities|String|Append "The socket name is already existing. Please check the Mesh :" "Socket \"" (Utilities|String|ToString(Name) _array_element_2) "\" at " "Mesh \"" (Utilities|GetDisplayName _array_element) "\"") true true "(R=1.000000,G=0.000000,B=0.000000,A=1.000000)" 5.0)
        (else
          (Utilities|Map|Add (Variables|Default|GetSocketNamesToMeshes) _array_element_2 _array_element))))))

(event EventShutdown)

(event EventWork)

(fn ConstructionScript
  (bind _returnvalue (Game|ConstructObjectfromClass "/Game/Zelda/InteractiveObj/BP_ConnectedObjCollector.BP_ConnectedObjCollector_C"))
  (bind _output_get (Variables|Default|SetConnectedObjCollector _returnvalue))
  (Default|AddNew _output_get self))

(fn GetMainPhysicsBody
  (return 0))