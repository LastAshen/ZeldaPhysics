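; BP_Swing is an interactive swing object that gains lift from its own physics-driven forward motion.
; Each tick, while the mesh moves along its forward vector, it adds upward acceleration scaled by that projected speed and RiseForceRate.
; The Work event only sets a Working flag, which Tick does not read.
; GetMainPhysicsBody returns the static mesh, and a disconnected debug push test remains in the graph.
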(event EventWork
  (Variables|Default|SetbWorking true))

(event EventTick
  (params (DeltaSeconds :type Float%20%28single-precision%29))
  (bind _staticmesh (Variables|Default|GetStaticMesh))
  (bind _staticmesh_2 (Variables|Default|GetStaticMesh))
  (bind _returnvalue (Math|Vector|GetForwardVector _staticmesh))
  (bind _returnvalue_2 (Transformation|GetComponentVelocity _staticmesh))
  ;[1 1 1] Tick
  (if (> (Math|Vector|DotProduct _returnvalue_2 _returnvalue) 0.0)
    (Physics|AddForce _staticmesh_2 (* (Math|Vector|GetUpVector _staticmesh_2) (* (Math|Vector|VectorLength (Math|Vector|ProjectVectorontoVector _returnvalue_2 _returnvalue)) (Variables|Default|GetRiseForceRate))) "None" true)))

(fn ConstructionScript
  (|CallParentFunction))

(fn GetMainPhysicsBody
  (return (Variables|Default|GetStaticMesh)))