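; BP_Tumbler is an interactive physics object that acts as a self-righting roly-poly toy while switched on.
; Work raises the mesh's mass scale and lowers its center of mass, and Shutdown restores both.
; While working, Tick applies angular impulses scaled by RotationForce, derived from the direction of world up relative to the mesh.
; An author note flags that heavy attached objects can still pull it over.
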(event EventTick
  (params (DeltaSeconds :type Float%20%28single-precision%29))
  (bind _staticmesh (Variables|Default|GetStaticMesh))
  (bind _rotationforce (Variables|Default|GetRotationForce))
  (bind _returnvalue (Transformation|GetWorldTransform _staticmesh))
  (bind _returnvalue_2 (Transformation|GetWorldLocation _staticmesh))
  (bind _returnvalue_3 (+ _returnvalue_2 "0.000000,0.000000,100.000000"))
  (bind _returnvalue_4 (Math|Rotator|FindRelativeLookatRotation _returnvalue _returnvalue_3))
  (bind _returnvalue_5 (Math|Rotator|GetRotationXVector _returnvalue_4))
  ;[1 1 1] 有待优化, 当连接的物体质量过大时，不倒翁会被拉到倾斜，
  (if (Variables|Default|GetbWorking)
    (Class|PrimitiveComponent|AddAngularImpulseinDegrees (Variables|Default|GetStaticMesh) (Math|Vector|MakeVector (* (.x _returnvalue_5) _rotationforce) (* (.y _returnvalue_5) _rotationforce) 0.0) "None" true)))

(event EventWork
  (Variables|Default|SetbWorking true)
  (Class|PrimitiveComponent|SetMassScale (Variables|Default|GetStaticMesh) "None" 3e+01)
  (Class|PrimitiveComponent|SetCenterOfMass (Variables|Default|GetStaticMesh) "0.000000,0.000000,-100.000000" "None"))

(event EventShutdown
  (Variables|Default|SetbWorking false)
  (Class|PrimitiveComponent|SetMassScale (Variables|Default|GetStaticMesh) "None" 1.0)
  (Class|PrimitiveComponent|SetCenterOfMass (Variables|Default|GetStaticMesh) "0, 0, 0" "None"))

(fn ConstructionScript
  (|CallParentFunction))

(fn GetMainPhysicsBody
  (return (Variables|Default|GetStaticMesh)))