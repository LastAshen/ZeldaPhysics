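; Player for a Zelda-style building mechanic that grabs, rotates, pushes and snaps together BP_ConnectableActor objects.
; A camera trace attaches the target to a movable sphere via a physics constraint; mouse input controls distance, rotation and working-state toggling.
; While holding, Tick sphere-traces for nearby connectables and marks nearest sockets.
; Connecting aligns sockets using inverse-transform composition, spawns a physics constraint and merges both objects' collections.
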(event EventBeginPlay
  ;[1 1 1] Beginplay
  (Input|EnableInput (Game|GetPlayerController 0)))

(event EventTick
  (params (DeltaSeconds :type Float%20%28single-precision%29))
  ;[1 1 1] Tick
  (if (Variables|Default|GetbOnFindingCandidateObj)
    (CallFunction|FindCandidateObj)))

(event Input|MouseEvents|MouseWheelAxis
  (params (AxisValue :type Float%20%28single-precision%29))
  (bind _returnvalue (* AxisValue 5e+01))
  (bind _camera (Variables|Default|GetCamera))
  (bind _sphere (Variables|Default|GetSphere))
  (bind _sphere_2 (Variables|Default|GetSphere))
  (bind _sphere_3 (Variables|Default|GetSphere))
  (bind _returnvalue_2 (Math|Vector|GetForwardVector _camera))
  (bind _returnvalue_3 (Transformation|GetWorldLocation _sphere))
  (bind _returnvalue_4 (Transformation|GetWorldLocation _camera))
  (bind _returnvalue_5 (* _returnvalue _returnvalue_2))
  (bind _returnvalue_6 (+ _returnvalue_3 _returnvalue_5))
  (bind _returnvalue_7 (- _returnvalue_6 _returnvalue_4))
  (if (Variables|Default|GetbShiftKeyDown)
    ;[1 1 1] UpDown Rotate
    (CallFunction|RotateGrabedObj (Math|Vector2D|MakeVector2D (* AxisValue 45.0) 0.0))
    (else
      ;[1 1 1] Distance Control
      (if (> (Math|Vector|DotProduct (Math|Vector|Normalize _returnvalue_7) _returnvalue_2) 0.0)
        (if (> (Math|Vector|VectorLength _returnvalue_7) 5e+01)
          (Transformation|AddWorldOffset _sphere_3 _returnvalue_5 false false)
          (else
            (Transformation|SetWorldLocation _sphere_3 (+ (Transformation|GetWorldLocation _sphere_2) (* (Math|Vector|GetForwardVector _sphere_2) 5e+01)) false false)))))))

(event Input|MouseEvents|LeftMouseButton
  (params (Key :type Key%20Structure :default "None"))
  (:Pressed
    (if (Variables|Default|GetbShiftKeyDown)
      (CallFunction|RotateGrabedObj "(X=0.000000,Y=45.000000)")
      (else
        ;[1 1 1] Grab
        (Utilities|IsValid (Variables|Default|GetGrabedComp)
          (:Is%20Valid
            (CallFunction|DropObj)
            (Variables|Default|SetbOnFindingCandidateObj false)
            (CallFunction|HideSocketShowPointer))
          (:Is%20Not%20Valid
            (bind _bfound (CallFunction|GrabObj))
            (Variables|Default|SetbOnFindingCandidateObj _bfound)))))))

(event Input|MouseEvents|RightMouseButton
  (params (Key :type Key%20Structure :default "None"))
  (bind _grabedsocket (Variables|Default|GetGrabedSocket))
  (bind _candidatesocket (Variables|Default|GetCandidateSocket))
  (bind _candidatesocket_2 (Variables|Default|GetCandidateSocket))
  (bind _grabedcomp (Variables|Default|GetGrabedComp))
  (bind _grabedsocket_2 (Variables|Default|GetGrabedSocket))
  (bind _candidatesocket_3 (Variables|Default|GetCandidateSocket))
  (bind _returnvalue (!= _grabedsocket ""))
  (bind _returnvalue_2 (!= _candidatesocket ""))
  (bind _returnvalue_3 (and _returnvalue _returnvalue_2))
  (:Pressed
    (if (Variables|Default|GetbShiftKeyDown)
      (CallFunction|RotateGrabedObj "(X=0.000000,Y=-45.000000)")
      (else
        (Utilities|IsValid (Variables|Default|GetGrabedComp)
          (:Is%20Valid
            (Variables|Default|SetbOnFindingCandidateObj false)
            (CallFunction|HideSocketShowPointer)
            (if (and (Utilities|IsValid (Variables|Default|GetGrabedComp)) (.bBlockingHit (Collision|BreakHitResult (Variables|Default|GetCandidateConnectObjInfo))))
              (Utilities|FlowControl|Sequence
                (:then_0
                  ;[1 1 1] Target Socket World Transform
                  (if _returnvalue_3
                    (bind _asbp_connectable_actor (Utilities|Casting|CastToBP_ConnectableActor (.HitActor (Collision|BreakHitResult (Variables|Default|GetCandidateConnectObjInfo)))))
                    (if (.ReturnValue (Utilities|Map|Find (Variables|/Game/Zelda/InteractiveObj/BP_ConnectableActor.BP_ConnectableActor_C|GetSocketNamesToMeshes _asbp_connectable_actor) _candidatesocket_2))
                      ;;[1 1 1] Seems problematic.
                      (Variables|Default|SetTargetSocketTfm (Math|Transform|MakeTransform (Transformation|GetSocketLocation (.Value (Utilities|Map|Find (Variables|/Game/Zelda/InteractiveObj/BP_ConnectableActor.BP_ConnectableActor_C|GetSocketNamesToMeshes _asbp_connectable_actor) _candidatesocket_2)) _candidatesocket_2) (Math|Rotator|MakeRotfromZ (Math|Vector|NegateVector (Math|Vector|GetUpVector (Transformation|GetSocketRotation (.Value (Utilities|Map|Find (Variables|/Game/Zelda/InteractiveObj/BP_ConnectableActor.BP_ConnectableActor_C|GetSocketNamesToMeshes _asbp_connectable_actor) _candidatesocket_2)) _candidatesocket_2))))))
                      (else
                        (Variables|Default|SetTargetTfm (Transformation|GetWorldTransform (.HitComponent (Collision|BreakHitResult (Variables|Default|GetCandidateConnectObjInfo)))) :!label _label)))
                    (else
                      (goto _label))))
                (:then_1
                  ;[1 1 1] Target Component World Transform
                  (if _returnvalue_3
                    (bind _asbp_connectable_actor_2 (Utilities|Casting|CastToBP_ConnectableActor (Components|GetOwner (Variables|Default|GetGrabedComp))))
                    (if (.ReturnValue (Utilities|Map|Find (Variables|/Game/Zelda/InteractiveObj/BP_ConnectableActor.BP_ConnectableActor_C|GetSocketNamesToMeshes _asbp_connectable_actor_2) _grabedsocket_2))
                      (Variables|Default|SetTargetTfm (Math|Transform|ComposeTransforms (Math|Transform|InvertTransform (Transformation|GetSocketTransform (.Value (Utilities|Map|Find (Variables|/Game/Zelda/InteractiveObj/BP_ConnectableActor.BP_ConnectableActor_C|GetSocketNamesToMeshes _asbp_connectable_actor_2) _grabedsocket_2)) _grabedsocket_2 "RTS_Component")) (Variables|Default|GetTargetSocketTfm)))
                      (else
                        (Variables|Default|SetTargetTfm (Transformation|GetWorldTransform (.HitComponent (Collision|BreakHitResult (Variables|Default|GetCandidateConnectObjInfo)))) :!label _label_2)))
                    (else
                      (goto _label_2))))
                (:then_2
                  ;[1 1 1] Connect
                  (bind _result (CallFunction|GetSocketMesh (Components|GetOwner (Variables|Default|GetGrabedComp)) (Variables|Default|GetGrabedSocket)))
                  (bind _result_2 (CallFunction|GetSocketMesh (.HitActor (Collision|BreakHitResult (Variables|Default|GetCandidateConnectObjInfo))) _candidatesocket_3))
                  (Components|MoveComponentTo _result (.location (Variables|Default|GetTargetTfm)) (.rotation (Variables|Default|GetTargetTfm)) false false 0.2 true)
                  (bind _returnvalue_4 (Game|SpawnActorfromClass "/Game/Zelda/InteractiveObj/BP_PhysicsConstraintTemplate.BP_PhysicsConstraintTemplate_C" (Math|Transform|MakeTransform (Transformation|GetSocketLocation _result_2 _candidatesocket_3) "0, 0, 0" "1.000000,1.000000,1.000000") "Undefined" "MultiplyWithRoot" 0 0))
                  (Class|PhysicsConstraintComponent|SetConstrainedComponents (Variables|/Script/Engine.PhysicsConstraintActor|GetConstraintComp _returnvalue_4) _result "None" _result_2 "None")
                  (Physics|SetPhysicsLinearVelocity _grabedcomp "0, 0, 0" false "None")
                  (Physics|SetPhysicsLinearVelocity _result_2 "0, 0, 0" false "None")
                  (bind _asbp_connectable_actor_3 (Utilities|Casting|CastToBP_ConnectableActor (Components|GetOwner _grabedcomp)))
                  (bind _asbp_connectable_actor_4 (Utilities|Casting|CastToBP_ConnectableActor (.HitActor (Collision|BreakHitResult (Variables|Default|GetCandidateConnectObjInfo)))))
                  (Utilities|MergeCollectionfromActors _asbp_connectable_actor_4 _asbp_connectable_actor_3
                    (:Next
                      (CallFunction|DropObj)
                      (Variables|Default|SetCandidateConnectObjInfo "")))))))
          (:Is%20Not%20Valid
            ;[1 1 1] Push
            (bind (_bhit _hitresult) (CallFunction|TraceObjfromMouse))
            (if _bhit
              (if (Physics|IsSimulatingPhysics (.HitComponent (Collision|BreakHitResult _hitresult)) (.BoneName (Collision|BreakHitResult _hitresult)))
                (Physics|AddForce (.HitComponent (Collision|BreakHitResult _hitresult)) (* (Math|Vector|GetForwardVector (Variables|Default|GetCamera)) (Variables|Default|GetPushForce)) (.BoneName (Collision|BreakHitResult _hitresult)) true)))))))))

(event Input|MouseEvents|MiddleMouseButton
  (params (Key :type Key%20Structure :default "None"))
  ;[1 1 1] Toggle Working State
  (:Pressed
    (bind (_bhit _hitresult) (CallFunction|TraceObjfromMouse))
    (if _bhit
      (bind _asbp_connectable_actor (Utilities|Casting|CastToBP_ConnectableActor (.HitActor (Collision|BreakHitResult _hitresult))))
      (Default|ToggleWorkingState (Variables|/Game/Zelda/InteractiveObj/BP_ConnectableActor.BP_ConnectableActor_C|GetConnectedObjCollector _asbp_connectable_actor)))))

(event Input|KeyboardEvents|LeftShift
  (params (Key :type Key%20Structure :default "None"))
  ;[1 1 1] Shift
  (:Pressed
    (Variables|Default|SetbShiftKeyDown true))
  (:Released
    (Variables|Default|SetbShiftKeyDown false)))

(event Input|KeyboardEvents|RightShift
  (params (Key :type Key%20Structure :default "None"))
  ;[1 1 1] Shift
  (:Pressed
    (Variables|Default|SetbShiftKeyDown true))
  (:Released
    (Variables|Default|SetbShiftKeyDown false)))

(event Input|KeyboardEvents|AnyKey
  (params (Key :type Key%20Structure :default "None"))
  ;[1 1 1] Close Tips
  (:Pressed
    (Utilities|FlowControl|DoOnce false
      (:Completed
        (bind _ashud_main (Utilities|Casting|CastToHUD_Main (HUD|GetHUD (Game|GetPlayerController 0))))
        (Default|CloseTips (Variables|/Game/Zelda/Game/HUD_Main.HUD_Main_C|GetMainView _ashud_main))))))

(event Input|MouseEvents|Mouse2D
  (params (AxisValue :type Vector :default "0, 0, 0"))
  (bind _returnvalue (Game|GetPlayerController 0))
  (bind _returnvalue_2 (Pawn|GetControlRotation _returnvalue :!class /Script/Engine.Controller))
  ;[1 1 1] Mouse View Control
  (Pawn|SetControlRotation _returnvalue (Math|Rotator|MakeRotator (.roll _returnvalue_2) (+ (.y AxisValue) (.pitch _returnvalue_2)) (+ (.x AxisValue) (.yaw _returnvalue_2)))))

(fn ConstructionScript)

(fn DropObj
  (Class|PhysicsConstraintComponent|BreakConstraint (Variables|Default|GetPhysicsConstraint))
  (Utilities|IsValid (Variables|Default|GetGrabedComp)
    (:Is%20Valid
      (Class|PrimitiveComponent|WakeAllRigidBodies (Variables|Default|GetGrabedComp))
      (Variables|Default|SetGrabedComp 0)
      (bind _ashud_main (Utilities|Casting|CastToHUD_Main (HUD|GetHUD (Game|GetPlayerController 0))))
      (Default|LoopRotateAnim (Variables|/Game/Zelda/Game/HUD_Main.HUD_Main_C|GetMainView _ashud_main) false))))

(fn FindCandidateObj
  (bind _sphere1 (Variables|Default|GetSphere1))
  (bind _grabedcomp (Variables|Default|GetGrabedComp))
  (bind _sphere2 (Variables|Default|GetSphere2))
  (bind _candidatesearchradius (Variables|Default|GetCandidateSearchRadius))
  (bind _grabedcomp_2 (Variables|Default|GetGrabedComp))
  (bind _grabedcomp_3 (Variables|Default|GetGrabedComp))
  (bind _returnvalue (Transformation|GetWorldLocation _grabedcomp))
  (bind _returnvalue_2 (Transformation|GetWorldLocation _grabedcomp_2))
  (Utilities|IsValid _grabedcomp_3
    (:Is%20Valid
      (bind _asbp_connectable_actor (Utilities|Casting|CastToBP_ConnectableActor (Components|GetOwner _grabedcomp_3)))
      (Variables|Default|SetCandidateConnectObjInfo "")
      (bind (_outhits _returnvalue_3) (Collision|MultiSphereTraceForObjects _returnvalue_2 _returnvalue_2 _candidatesearchradius (Utilities|Array|MakeArray "ObjectTypeQuery4") false (Variables|/Game/Zelda/InteractiveObj/BP_ConnectedObjCollector.BP_ConnectedObjCollector_C|GetConnectedObjects (Variables|/Game/Zelda/InteractiveObj/BP_ConnectableActor.BP_ConnectableActor_C|GetConnectedObjCollector _asbp_connectable_actor)) "None" true "(R=1.000000,G=0.000000,B=0.611989,A=0.000000)"))
      (Rendering|Debug|DrawDebugSphere _returnvalue_2 _candidatesearchradius 18 (select _returnvalue_3 "(R=0.097830,G=1.000000,B=0.117439,A=1.000000)" "(R=1.000000,G=0.012392,B=0.872994,A=1.000000)") 0.0 0.3)
      (if _returnvalue_3
        ;[1 1 1] Find the Nearest Obj
        (for _array_element _outhits
          (if (not (.bBlockingHit (Collision|BreakHitResult (Variables|Default|GetCandidateConnectObjInfo))))
            (Variables|Default|SetCandidateConnectObjInfo _array_element :!label _label)
            (elif (and (> (Class|KismetMathLibrary|VectorDistanceSquared (Transformation|GetWorldLocation (.HitComponent (Collision|BreakHitResult (Variables|Default|GetCandidateConnectObjInfo)))) _returnvalue) (Class|KismetMathLibrary|VectorDistanceSquared _returnvalue (Transformation|GetWorldLocation (.HitComponent (Collision|BreakHitResult _array_element))))) (Class|GameplayStatics|ObjectIsA (.HitActor (Collision|BreakHitResult _array_element)) "/Game/Zelda/InteractiveObj/BP_ConnectableActor.BP_ConnectableActor_C"))
              (goto _label))))
        ;[1 1 1] Show
        (if (.bBlockingHit (Collision|BreakHitResult (Variables|Default|GetCandidateConnectObjInfo)))
          (Utilities|FlowControl|Sequence
            (:then_0
              (bind _asbp_connectable_actor_2 (Utilities|Casting|CastToBP_ConnectableActor (.HitActor (Collision|BreakHitResult (Variables|Default|GetCandidateConnectObjInfo)))))
              (bind _socketname (CallFunction|FindNearestSocket _asbp_connectable_actor_2 (.ImpactPoint (Collision|BreakHitResult (Variables|Default|GetCandidateConnectObjInfo)))))
              (bind _output_get (Variables|Default|SetCandidateSocket _socketname))
              (if (!= _output_get "")
                (Transformation|SetWorldLocation _sphere1 (Transformation|GetSocketLocation (.Value (Utilities|Map|Find (Variables|/Game/Zelda/InteractiveObj/BP_ConnectableActor.BP_ConnectableActor_C|GetSocketNamesToMeshes _asbp_connectable_actor_2) (Variables|Default|GetCandidateSocket))) (Variables|Default|GetCandidateSocket)) false false)
                (Rendering|SetVisibility _sphere1 true false)
                (else
                  (Rendering|SetVisibility (Variables|Default|GetSphere1) false false))))
            (:then_3
              (bind _asbp_connectable_actor_3 (Utilities|Casting|CastToBP_ConnectableActor (Components|GetOwner (Variables|Default|GetGrabedComp))))
              (bind _socketname_2 (CallFunction|FindNearestSocket _asbp_connectable_actor_3 (.ImpactPoint (Collision|BreakHitResult (Variables|Default|GetCandidateConnectObjInfo)))))
              (bind _output_get_2 (Variables|Default|SetGrabedSocket _socketname_2))
              (if (!= _output_get_2 "")
                (Transformation|SetWorldLocation _sphere2 (Transformation|GetSocketLocation (.Value (Utilities|Map|Find (Variables|/Game/Zelda/InteractiveObj/BP_ConnectableActor.BP_ConnectableActor_C|GetSocketNamesToMeshes _asbp_connectable_actor_3) (Variables|Default|GetGrabedSocket))) (Variables|Default|GetGrabedSocket)) false false)
                (Rendering|SetVisibility _sphere2 true false)
                (else
                  (Rendering|SetVisibility (Variables|Default|GetSphere2) false false)))))
          (else
            (CallFunction|HideSocketShowPointer :!label _label_2)
            (Variables|Default|SetCandidateSocket "None")
            (Variables|Default|SetGrabedSocket "None")))
        (else
          (Variables|Default|SetCandidateConnectObjInfo "" :!label _label_3)
          (goto _label_2))))
    (:Is%20Not%20Valid
      (goto _label_3))))

(fn GrabObj
  (bind (_bhit _hitresult) (CallFunction|TraceObjfromMouse))
  (if (and _bhit (Class|GameplayStatics|ObjectIsA (.HitActor (Collision|BreakHitResult _hitresult)) "/Game/Zelda/InteractiveObj/BP_ConnectableActor.BP_ConnectableActor_C"))
    (bind _output_get (Variables|Default|SetGrabedComp (.HitComponent (Collision|BreakHitResult _hitresult))))
    (Transformation|SetWorldLocation (Variables|Default|GetSphere) (.Location (Collision|BreakHitResult _hitresult)) false true)
    (Class|PhysicsConstraintComponent|SetConstrainedComponents (Variables|Default|GetPhysicsConstraint) (Variables|Default|GetSphere) "None" _output_get (.HitBoneName (Collision|BreakHitResult _hitresult)))
    (bind _ashud_main (Utilities|Casting|CastToHUD_Main (HUD|GetHUD (Game|GetPlayerController 0)))
      (:then
        (Default|LoopRotateAnim (Variables|/Game/Zelda/Game/HUD_Main.HUD_Main_C|GetMainView _ashud_main) true))
      (:CastFailed
        _))
    (return true)
    (else
      (return false))))

(fn TraceObjfromMouse
  (bind _camera (Variables|Default|GetCamera))
  (bind _returnvalue (Transformation|GetWorldLocation _camera))
  (bind (_outhit _returnvalue_2) (Collision|LineTraceForObjects _returnvalue (+ _returnvalue (* (Math|Vector|GetForwardVector _camera) 1e+05)) (Utilities|Array|MakeArray "ObjectTypeQuery2" "ObjectTypeQuery4") false 0 "None"))
  (return _returnvalue_2 _outhit))

(fn FindNearestSocket
  (params (Src :type BP%20Connectable%20Actor%20Object%20Reference) (DestPoint :type Vector))
  (bind _socketnamestomeshes (Variables|/Game/Zelda/InteractiveObj/BP_ConnectableActor.BP_ConnectableActor_C|GetSocketNamesToMeshes Src))
  (LocalVariables|SetNearestSocket "None")
  (bind _keys (Utilities|Map|Keys _socketnamestomeshes))
  (for _array_element _keys
    (if (or (== (LocalVariables|GetNearestSocket) "") (> (Math|Vector|Distance(Vector) (Transformation|GetSocketLocation (.Value (Utilities|Map|Find _socketnamestomeshes _array_element)) (LocalVariables|GetNearestSocket)) DestPoint) (Math|Vector|Distance(Vector) (Transformation|GetSocketLocation (.Value (Utilities|Map|Find _socketnamestomeshes _array_element)) _array_element) DestPoint)))
      (LocalVariables|SetNearestSocket _array_element)))
  (return (LocalVariables|GetNearestSocket)))

(fn HideSocketShowPointer
  ;[1 1 1] Hide
  (Rendering|SetVisibility (Variables|Default|GetSphere1) false false)
  (Rendering|SetVisibility (Variables|Default|GetSphere2) false false))

(fn GetSocketMesh
  (params (Actor :type Actor%20Object%20Reference) (SocketName :type Name))
  (bind _asbp_connectable_actor (Utilities|Casting|CastToBP_ConnectableActor Actor)
    (:then
      (if (.ReturnValue (Utilities|Map|Find (Variables|/Game/Zelda/InteractiveObj/BP_ConnectableActor.BP_ConnectableActor_C|GetSocketNamesToMeshes _asbp_connectable_actor) SocketName))
        (return (.Value (Utilities|Map|Find (Variables|/Game/Zelda/InteractiveObj/BP_ConnectableActor.BP_ConnectableActor_C|GetSocketNamesToMeshes _asbp_connectable_actor) SocketName)))
        (else
          _)))
    (:CastFailed
      _))
  (return 0))

(fn RotateGrabedObj
  (params (AddAngels :type Vector%202D%20Structure))
  (bind _camera (Variables|Default|GetCamera))
  (bind _grabedcomp (Variables|Default|GetGrabedComp))
  (Utilities|IsValid _grabedcomp
    (:Is%20Valid
      (Transformation|SetWorldRotation (Variables|Default|GetGrabedComp) (Math|Rotator|CombineRotators (Math|Rotator|CombineRotators (Transformation|GetWorldRotation _grabedcomp) (Math|Vector|RotatorfromAxisandAngle (Math|Vector|GetRightVector _camera) (.x AddAngels))) (Math|Vector|RotatorfromAxisandAngle (Math|Vector|GetUpVector _camera) (.y AddAngels))) false false))))