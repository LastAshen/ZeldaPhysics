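; BP_RadialForce is a physics test actor that applies a radial force among a group of constrained meshes.
; The construction script builds twenty scaled-down static meshes, stores them in Receivers, and gives each a physics constraint with only the first component set.
; Two seconds after BeginPlay, it adds a manually attached RadialForceComponent, using a random receiver's relative location as its transform location.
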(event EventBeginPlay
  (Utilities|FlowControl|Delay 2.0)
  (AddComponent|AddRadialForceComponent true (Math|Transform|MakeTransform (Variables|/Script/Engine.SceneComponent|GetRelativeLocation (.OutItem (Utilities|Array|Random (Variables|Default|GetReceivers)))) "0, 0, 0" "1.000000,1.000000,1.000000")))

(fn ConstructionScript
  (for _index (range 0 19)
    (bind _returnvalue (AddComponent|AddStaticMeshComponent false (Math|Transform|MakeTransform "0, 0, 0" "0, 0, 0" "0.300000,0.300000,0.300000")))
    (Utilities|Array|Add (Variables|Default|GetReceivers) _returnvalue)
    (bind _returnvalue_2 (AddComponent|AddPhysicsConstraintComponent false))
    (Class|PhysicsConstraintComponent|SetConstrainedComponents _returnvalue_2 _returnvalue "None" 0 "None")))